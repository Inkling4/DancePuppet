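; Medium enemy puppet AI character that chases the player once spotted and performs a basic melee attack on reaching them.
; PuppetSenses pawn sensing sets IsPlayerSeen and triggers FollowPlayer, which runs AI MoveTo toward the player character.
; On arrival it plays a montage and calls BasicAttack, with CanAttack cleared but never checked.
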(event `self.PuppetSenses.OnSeePawn`
  (params (Pawn :type "Pawn Object Reference"))
  (set `self.isPlayerSeen` true)
  (`self.FollowPlayer`))

(event `FollowPlayer`
  (if (`self.isPlayerSeen`)
    (`|AIMoveTo` self (0.0 0.0 0.0) (`GameplayStatics.GetPlayerCharacter` 0) 80.0
      (:`OnSuccess`
        (if true
          (set `self.canAttack` false)
          (`self.PlayAnimMontage` null)
          (`self.BasicAttack`))))))

(fn `UserConstructionScript`)