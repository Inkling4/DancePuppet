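; Player puppet Blueprint, a medium variant by name, that turns to face the point under the mouse cursor.
; Each Tick, if player controller 0 is valid, it traces under the cursor on the Visibility channel using complex collision.
; The look-at target keeps the actor's own height, so the rotation stays horizontal.
; Death, BeginPlay, overlap and construction hooks are empty.
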(event `self.OnDeath`)

(event `self.ReceiveTick`
  (params (DeltaSeconds :type "Float (single-precision)"))
  (bind _returnvalue (`self.K2_GetActorLocation`))
  (if (`KismetSystemLibrary.IsValid` (`GameplayStatics.GetPlayerController` 0))
    (`self.K2_SetActorRotation` (`KismetMathLibrary.FindLookAtRotation` _returnvalue (`KismetMathLibrary.MakeVector` (.x (`.Location` (`GameplayStatics.BreakHitResult` (`PlayerController.GetHitResultUnderCursorByChannel` (`GameplayStatics.GetPlayerController` 0) "TraceTypeQuery1" true)))) (.y (`.Location` (`GameplayStatics.BreakHitResult` (`PlayerController.GetHitResultUnderCursorByChannel` (`GameplayStatics.GetPlayerController` 0) "TraceTypeQuery1" true)))) (.z _returnvalue))))))

(fn `UserConstructionScript`)