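; Player puppet character for the fight game that turns to face the mouse cursor and handles its own death.
; Each Tick, until game over, it traces under the cursor on the Visibility channel and yaws toward that point at its own height.
; OnDeath shows the death screen, stops regen, flags game over on itself and BP_FightGameMode, zeroes knockback and disables player input.
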(event `self.ReceiveBeginPlay`
  (set `self.IsGameOver` false))

(event `self.OnDeath`
  (bind _returnvalue (`|CreateWidget` "/Game/Blueprints/WBP_DeathScreen.WBP_DeathScreen_C"))
  (`UserWidget.AddToViewport` _returnvalue 0)
  (set `self.bRegenEnabled` false)
  (bind _asbp_fight_game_mode (cast `/Game/Blueprints/BP_FightGameMode` (`GameplayStatics.GetGameMode`)))
  (set `/Game/Blueprints/BP_FightGameMode.IsGameOver` true _asbp_fight_game_mode)
  (set `self.KnockbackMult` 0.0)
  (`self.DisableInput` (`GameplayStatics.GetPlayerController` 0))
  (set `self.IsGameOver` true))

(event `self.ReceiveTick`
  (params (DeltaSeconds :type "Float (single-precision)"))
  (bind _returnvalue (`self.K2_GetActorLocation`))
  ; Looks at mouse
  (if (`self.IsGameOver`)
    _
    (elif (`KismetSystemLibrary.IsValid` (`GameplayStatics.GetPlayerController` 0))
      (`self.K2_SetActorRotation` (`KismetMathLibrary.FindLookAtRotation` _returnvalue (`KismetMathLibrary.MakeVector` (.x (`.Location` (`GameplayStatics.BreakHitResult` (`PlayerController.GetHitResultUnderCursorByChannel` (`GameplayStatics.GetPlayerController` 0) "TraceTypeQuery1" true)))) (.y (`.Location` (`GameplayStatics.BreakHitResult` (`PlayerController.GetHitResultUnderCursorByChannel` (`GameplayStatics.GetPlayerController` 0) "TraceTypeQuery1" true)))) (.z _returnvalue)))))))

(fn `UserConstructionScript`)